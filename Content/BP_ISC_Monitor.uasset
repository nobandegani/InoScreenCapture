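; BP_ISC_Monitor is a monitor Blueprint that displays a supplied texture through a widget component.
; Its Init event creates a WBP_ISC_Monitor widget for the first player controller, passing itself as a reference, and assigns it to the component.
; It then forwards the monitor data and texture to that widget and sizes the component's draw area to the monitor's width and height.
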(event `Init`
  (params (Monitor :type "ISC_MonitorInfo Structure (by ref)") (Texture :type "Texture2D Object Reference (by ref)"))
  (bind (_index _id _width _height) (break `ISC_MonitorInfo` Monitor))
  (bind _widget (`self.Widget`))
  (bind _returnvalue (`|CreateWidget` "/InoScreenCapture/WBP_ISC_Monitor.WBP_ISC_Monitor_C" (`GameplayStatics.GetPlayerController` 0) self))
  (bind _output_get (set `self.UI Ref` _returnvalue))
  (`WidgetComponent.SetWidget` _widget _output_get)
  (`/InoScreenCapture/WBP_ISC_Monitor.Init` _output_get Monitor Texture)
  (`WidgetComponent.SetDrawSize` _widget (`KismetMathLibrary.MakeVector2D` (`KismetMathLibrary.Conv_IntToDouble` _width) (`KismetMathLibrary.Conv_IntToDouble` _height))))

(fn `UserConstructionScript`)