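; BP_ISC_IntegrationTest is an integration test actor for the InoScreenCapture subsystem that displays captured monitors in the level.
; On BeginPlay it registers a monitor-init callback, then starts screen capture for every monitor ID the subsystem reports.
; Each callback spawns a BP_ISC_Monitor, offset along X by the count of existing ones, and initializes it with that monitor's info and texture.
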(event `self.ReceiveBeginPlay`
  (bind _returnvalue (subsystem `InoScreenCaptureSubSystem`))
  (add `InoScreenCaptureSubSystem.MonitorCaptureInitCallback` _returnvalue (delegate `MonitorCaptureInitCallback_Event`))
  (bind _returnvalue_2 (`InoScreenCaptureSubSystem.GetMonitors` _returnvalue))
  (bind _keys (`BlueprintMapLibrary.Map_Keys` _returnvalue_2))
  (`InoScreenCaptureSubSystem.InitScreenCapture` _returnvalue 13 _keys false false))

(event `MonitorCaptureInitCallback_Event`
  (params (MonitorInfo :type "ISC_MonitorInfo Structure (by ref)") (Texture2D :type "Texture2D Object Reference"))
  (bind _outactors (`GameplayStatics.GetAllActorsOfClass` "/InoScreenCapture/BP_ISC_Monitor.BP_ISC_Monitor_C"))
  (bind _returnvalue (`|SpawnActorFromClass` "/InoScreenCapture/BP_ISC_Monitor.BP_ISC_Monitor_C" (`KismetMathLibrary.MakeTransform` (`KismetMathLibrary.MakeVector` (`KismetMathLibrary.Conv_IntToDouble` (* 500 (`KismetArrayLibrary.Array_Length` _outactors))))) "Undefined" "MultiplyWithRoot" null null))
  (`/InoScreenCapture/BP_ISC_Monitor.Init` _returnvalue MonitorInfo Texture2D))

(fn `UserConstructionScript`)